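; Enemy Blueprint that wanders the navmesh and chases pawns it sees, using event graph logic with no behavior tree.
; Roaming moves to a random navigable point around its current location and calls itself again on success or failure.
; PawnSensing sightings start a move toward the seen pawn and reset a one-second retriggerable delay, which resumes roaming once sightings stop.
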(event `self.ReceiveBeginPlay`
  (`self.Roaming`))

(event `Roaming`
  (bind _randomlocation (`NavigationSystemV1.K2_GetRandomLocationInNavigableRadius` (`self.K2_GetActorLocation`) 2000.0 null null))
  (`|AIMoveTo` self _randomlocation null
    (:`OnSuccess`
      _)
    (:`OnFail`
      _))
  (`self.Roaming`))

(event `self.PawnSensing.OnSeePawn`
  (params (Pawn :type "Pawn Object Reference"))
  (`|ExecutionSequence`
    (:`then_0`
      (`|AIMoveTo` self (0.0 0.0 0.0) Pawn))
    (:`then_1`
      (`KismetSystemLibrary.RetriggerableDelay` 1.0)
      (`self.Roaming`))))

(fn `UserConstructionScript`)