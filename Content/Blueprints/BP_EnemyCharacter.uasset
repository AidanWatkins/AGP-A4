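; BP_EnemyCharacter is an enemy character with a gun mesh and pawn-sensing hooks for following the player.
; Gun visibility follows HasWeapon on BeginPlay and can be toggled through EquipWeaponGraphical.
; Seeing a pawn sets HasSeenPlayer to false, then calls FollowPlayer, which only runs AI MoveTo toward player 0 when that flag is true.
; As wired, sighting a pawn therefore never starts the chase.
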(event `self.ReceiveBeginPlay`
  (bind _returnvalue (`self.HasWeapon`))
  (`SceneComponent.SetVisibility` (`self.GunMesh`) _returnvalue false))

(event `self.EquipWeaponGraphical`
  (params (bEquipWeapon :type Boolean))
  (`SceneComponent.SetVisibility` (`self.GunMesh`) bEquipWeapon false))

(event `self.PawnSensingComponent.OnSeePawn`
  (params (Pawn :type "Pawn Object Reference"))
  (set `self.hasSeenPlayer` false)
  (`self.FollowPlayer`))

(event `FollowPlayer`
  (if (`self.hasSeenPlayer`)
    (`|AIMoveTo` self (0.0 0.0 0.0) (`GameplayStatics.GetPlayerCharacter` 0))))

(fn `UserConstructionScript`)